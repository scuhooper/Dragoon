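; Enemy agent Blueprint that equips itself with a sheathed sword when play begins.
; BeginPlay spawns a SwordBP, stores it as Sword, snaps it to the mesh's Sword_Sheathe socket and makes the agent its owner.
; The construction script sets the mesh to overlap on the custom GameTraceChannel1 collision channel.
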(event EventBeginPlay
  (bind _returnvalue (Game|SpawnActorfromClass "/Game/Blueprints/SwordBP.SwordBP_C" (Variables|Default|GetSwordTransform) "Undefined" 0 0))
  (bind _output_get (Variables|Default|Setsword _returnvalue))
  (Transformation|AttachComponentToComponent _output_get (Variables|Character|GetMesh) "Sword_Sheathe" "SnapToTarget" "SnapToTarget" "SnapToTarget" false)
  (Actor|SetOwner (Variables|Default|Getsword) self))

(event Collision|EventActorBeginOverlap
  (params (OtherActor :type Actor%20Object%20Reference)))

(event EventTick
  (params (DeltaSeconds :type Float%20%28single-precision%29)))

(fn ConstructionScript
  (Collision|SetCollisionResponsetoChannel (Variables|Character|GetMesh) "ECC_GameTraceChannel1" "ECR_Overlap"))